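; BP_NavPoint is a helper Blueprint that serves as a visual navigation point marker which can be shown or hidden.
; Its Hide and Show events toggle visibility on the LowerCone, UpperCone, Cone and Center components, without propagating to children.
; It has no other logic, as BeginPlay, overlap, Tick and the construction script are all empty.
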(event `self.ReceiveTick`
  (params (DeltaSeconds :type "Float (single-precision)")))

(event `Hide`
  (`SceneComponent.SetVisibility` (`self.LowerCone`) false false)
  (`SceneComponent.SetVisibility` (`self.UpperCone`) false false)
  (`SceneComponent.SetVisibility` (`self.Cone`) false false)
  (`SceneComponent.SetVisibility` (`self.center`) false false))

(event `Show`
  (`SceneComponent.SetVisibility` (`self.LowerCone`) true false)
  (`SceneComponent.SetVisibility` (`self.UpperCone`) true false)
  (`SceneComponent.SetVisibility` (`self.Cone`) true false)
  (`SceneComponent.SetVisibility` (`self.center`) true false))

(fn `UserConstructionScript`)