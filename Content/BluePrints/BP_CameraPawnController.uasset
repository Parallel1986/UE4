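; Player controller for a vessel-commanding strategy game, handling camera navigation, vessel placement, selection and orders.
; On BeginPlay it spawns the placement ghost, call manager, player data and nav point, and creates the HUD.
; In placement mode the ghost follows the cursor and clicks queue or cancel it; otherwise clicks select vessels or set targets.
; Camera supports axis and screen-edge movement, zoom and gated rotation, with pan speed scaled by zoom.
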(event `self.ReceiveBeginPlay`
  (bind _returnvalue (`KismetMathLibrary.MakeTransform` (0.0 0.0 0.0)))
  ;[1 1 1] Initialising
  ;;[1 1 1] Getting Camera Reference
  (bind _asbp_camera_pawn (cast `/Game/BluePrints/BP_CameraPawn` (`GameplayStatics.GetPlayerPawn` 0)))
  (set `self.refCameraPawn` _asbp_camera_pawn)
  (bind _returnvalue_2 (`|SpawnActorFromClass` "/Game/BluePrints/Vessels/BP_BaseVessel.BP_BaseVessel_C" (`KismetMathLibrary.MakeTransform` (0.0 0.0 0.0)) "AlwaysSpawn" "OverrideRootScale" null self null))
  (set `self.refBaseVessel` _returnvalue_2)
  (bind _returnvalue_3 (`|SpawnActorFromClass` "/Game/BluePrints/VesselsConstruction/BP_VesselGhost.BP_VesselGhost_C" (`KismetMathLibrary.MakeTransform` (0.0 0.0 0.0)) "AlwaysSpawn" "OverrideRootScale" null self null))
  (set `self.refVesselGhost` _returnvalue_3)
  (bind _returnvalue_4 (`|SpawnActorFromClass` "/Game/BluePrints/VesselsConstruction/BP_VesselCallManager.BP_VesselCallManager_C" (`KismetMathLibrary.MakeTransform` (0.0 0.0 0.0)) "AlwaysSpawn" "OverrideRootScale" null null))
  (set `self.refVesselCallManager` _returnvalue_4)
  ;;[1 1 1] Creating HUD
  (bind _returnvalue_5 (`|CreateWidget` "/Game/BluePrints/HUDS/BP_HUDWidget.BP_HUDWidget_C" null self (`self.refVesselGhost`)))
  (set `self.refHUD` _returnvalue_5)
  (bind _returnvalue_6 (`|SpawnActorFromClass` "/Game/BluePrints/BP_PlayerData.BP_PlayerData_C" _returnvalue "AlwaysSpawn" "OverrideRootScale" null null))
  (set `self.refPlayerData` _returnvalue_6)
  (bind _returnvalue_7 (`|SpawnActorFromClass` "/Game/BluePrints/Helpers/BP_NavPoint.BP_NavPoint_C" _returnvalue "Undefined" "OverrideRootScale" self null null))
  (bind _output_get (set `self.NavPos` _returnvalue_7))
  (`/Game/BluePrints/Helpers/BP_NavPoint.Hide` _output_get)
  (`WidgetBlueprintLibrary.SetInputMode_GameAndUIEx` self null "LockAlways" false)
  (`UserWidget.AddToViewport` (`self.refHUD`) 0))

(event `self.ReceiveTick`
  (params (DeltaSeconds :type "Float (single-precision)"))
  ;[1 1 1] Ticking
  (`|ExecutionSequence`
    (:`then_0`
      (if (`self.isPlacingVessel`)
        (if (!= (`self.refVesselGhost`) null)
          (bind _location (`/Game/BluePrints/Fuctions/Functions.SetCursorWorldPosition` self (`self.SetSightDistance`)))
          (`/Game/BluePrints/VesselsConstruction/BP_VesselGhost.Set Cursor Position` (`self.refVesselGhost`) _location))))))

(event `InputAxis|MoveRight`
  (params (AxisValue :type "Float (single-precision)"))
  (bind _returnvalue (`self.GetTransform` (`self.refCameraPawn`)))
  ;[1 1 1] Camera Movement
  ;;[1 1 1] MovementY
  (if (not (`self.isDisabledCamNav`))
    (`self.K2_SetActorTransform` (`self.refCameraPawn`) (`KismetMathLibrary.MakeTransform` (`KismetMathLibrary.MakeVector` (.x (+ (`KismetMathLibrary.TransformDirection` _returnvalue (`KismetMathLibrary.MakeVector` 0.0 (* AxisValue (`self.CalculateSensitivity`)))) (.location _returnvalue))) (.y (+ (`KismetMathLibrary.TransformDirection` _returnvalue (`KismetMathLibrary.MakeVector` 0.0 (* AxisValue (`self.CalculateSensitivity`)))) (.location _returnvalue))) 100.0) (.rotation _returnvalue) (.scale _returnvalue)) false false)))

(event `InputAxis|MoveUp`
  (params (AxisValue :type "Float (single-precision)"))
  (bind _returnvalue (`self.GetTransform` (`self.refCameraPawn`)))
  ;[1 1 1] Camera Movement
  ;;[1 1 1] MovementX
  (if (not (`self.isDisabledCamNav`))
    (`self.K2_SetActorTransform` (`self.refCameraPawn`) (`KismetMathLibrary.MakeTransform` (`KismetMathLibrary.MakeVector` (.x (+ (`KismetMathLibrary.TransformDirection` _returnvalue (`KismetMathLibrary.MakeVector` (* AxisValue (`self.CalculateSensitivity`)))) (.location _returnvalue))) (.y (+ (`KismetMathLibrary.TransformDirection` _returnvalue (`KismetMathLibrary.MakeVector` (* AxisValue (`self.CalculateSensitivity`)))) (.location _returnvalue))) 100.0) (.rotation _returnvalue) (.scale _returnvalue)) false false)))

(event `Key|LeftMouseButton`
  (params (Key :type "Key Structure"))
  (:`Pressed`
    ;[1 1 1] Placing Vessels
    (if (`self.isPlacingVessel`)
      (bind _vesselstructure (`/Game/BluePrints/VesselsConstruction/BP_VesselGhost.GetVesselStruct` (`self.refVesselGhost`)))
      (`/Game/BluePrints/VesselsConstruction/BP_VesselCallManager.VesselCallQueue` (`self.refVesselCallManager`) _vesselstructure)
      (`/Game/BluePrints/VesselsConstruction/BP_VesselGhost.KillGhost` (`self.refVesselGhost`))
      (else
        ;[1 1 1] Selection
        (bind _asbp_base_vessel (cast `/Game/BluePrints/Vessels/BP_BaseVessel` (`.HitActor` (`GameplayStatics.BreakHitResult` (`self.GetHitResultUnderCursorForObjects` (`self.EnumSelectableObjects`)))))
          (:`then`
            (if (!= _asbp_base_vessel null)
              (`/Game/BluePrints/BP_PlayerData.SelectVessel` (`self.refPlayerData`) _asbp_base_vessel)))
          (:`CastFailed`
            (`KismetSystemLibrary.PrintString` "FailedCastVessel")
            (`/Game/BluePrints/BP_PlayerData.DeselectAll` (`self.refPlayerData`))))))))

(event `InputAction|ZoomIn`
  (params (Key :type "Key Structure"))
  (bind _springarm (`/Game/BluePrints/BP_CameraPawn.SpringArm` (`self.refCameraPawn`)))
  ;[1 1 1] Camera Movement
  ;;[1 1 1] Zoom In
  (:`Pressed`
    (if (not (`self.isDisabledCamNav`))
      (set `SpringArmComponent.TargetArmLength` (`KismetMathLibrary.FClamp` (- (`SpringArmComponent.TargetArmLength` _springarm) (`self.ZoomSensitivity`)) (`self.MinZoom`) (`self.MaxZoom`)) _springarm))))

(event `Key|LeftShift`
  (params (Key :type "Key Structure"))
  ;[1 1 1] Camera Movement
  ;;[1 1 1] Fast Movement
  (:`Pressed`
    (set `self.MoveMultiplyer` 2.0))
  (:`Released`
    (set `self.MoveMultiplyer` 1.0)))

(event `InputAxisKey|MouseX`
  (params (AxisValue :type "Float (single-precision)"))
  ;[1 1 1] Camera Movement
  ;;[1 1 1] Edge Movement
  (if (not (`self.isDisabledCamNav`))
    (bind (_deltaxspeed _deltayspeed) (`self.EdgeMovement` :!label _label))
    (`self.K2_AddActorLocalOffset` (`self.refCameraPawn`) (`KismetMathLibrary.MakeVector` _deltaxspeed _deltayspeed) true false)))

(event `InputAction|AddSelection`
  (params (Key :type "Key Structure"))
  (:`Pressed`
    ;[1 1 1] Adding Selection
    (if (not (`self.isPlacingVessel`))
      (bind _asbp_base_vessel (cast `/Game/BluePrints/Vessels/BP_BaseVessel` (`.HitActor` (`GameplayStatics.BreakHitResult` (`self.GetHitResultUnderCursorForObjects` (`self.EnumSelectableObjects`))))))
      (if (!= _asbp_base_vessel null)
        (`/Game/BluePrints/BP_PlayerData.ToggleSelectionOfVessel` (`self.refPlayerData`) _asbp_base_vessel)))))

(event `InputAction|ZoomOut`
  (params (Key :type "Key Structure"))
  (bind _springarm (`/Game/BluePrints/BP_CameraPawn.SpringArm` (`self.refCameraPawn`)))
  ;[1 1 1] Camera Movement
  ;;[1 1 1] Zoom Out
  (:`Pressed`
    (if (not (`self.isDisabledCamNav`))
      (set `SpringArmComponent.TargetArmLength` (`KismetMathLibrary.FClamp` (+ (`SpringArmComponent.TargetArmLength` _springarm) (`self.ZoomSensitivity`)) (`self.MinZoom`) (`self.MaxZoom`)) _springarm))))

(event `InputAxisKey|MouseY`
  (params (AxisValue :type "Float (single-precision)"))
  ;[1 1 1] Camera Movement
  ;;[1 1 1] Edge Movement
  (if (not (`self.isDisabledCamNav`))
    (goto _label :!via `MoveY`)))

(event `InputAxisKey|MouseX`
  (params (AxisValue :type "Float (single-precision)"))
  ;[1 1 1] Camera Movement
  ;;[1 1 1] Camera Rotation
  (if (not (`self.isDisabledCamNav`))
    (`/Engine/EditorBlueprintResources/StandardMacros.Gate` true :!label _label_2
      (:`Exit`
        (`self.K2_SetActorRotation` (`self.refCameraPawn`) (`KismetMathLibrary.MakeRotator` (.roll (`self.K2_GetActorRotation` (`self.refCameraPawn`))) (.pitch (`self.K2_GetActorRotation` (`self.refCameraPawn`))) (+ (.yaw (`self.K2_GetActorRotation` (`self.refCameraPawn`))) (* AxisValue (`self.RotateSensitivity`)))) false)))))

(event `Key|RightMouseButton`
  (params (Key :type "Key Structure"))
  (bind _navpos (`self.NavPos`))
  (:`Pressed`
    ;[1 1 1] Cancel Placing
    (if (`self.isPlacingVessel`)
      (`/Game/BluePrints/VesselsConstruction/BP_VesselGhost.KillGhost` (`self.refVesselGhost`))
      (set `self.isPlacingVessel` false)
      (else
        ;[1 1 1] Setting Order
        (bind _asbp_base_vessel (cast `/Game/BluePrints/Vessels/BP_BaseVessel` (`.HitActor` (`GameplayStatics.BreakHitResult` (`self.GetHitResultUnderCursorForObjects` (`self.EnumSelectableObjects`)))))
          (:`then`
            (`/Game/BluePrints/BP_PlayerData.SetTarget` (`self.refPlayerData`) _asbp_base_vessel))
          (:`CastFailed`
            (bind _location (`/Game/BluePrints/Fuctions/Functions.SetCursorWorldPosition` self (* (`self.SightDistance`) 20.0)))
            (`SceneComponent.K2_SetWorldLocation` (`Actor.RootComponent` _navpos) _location false true)
            (`/Game/BluePrints/BP_PlayerData.SetTarget` (`self.refPlayerData`) _navpos)))))))

(event `InputAction|Panning`
  (params (Key :type "Key Structure"))
  ;[1 1 1] Camera Movement
  ;;[1 1 1] Camera Rotation
  (:`Pressed`
    (goto _label_2 :!via `Open`))
  (:`Released`
    (goto _label_2 :!via `Close`)))

(event `InputAxisKey|MouseY`
  (params (AxisValue :type "Float (single-precision)"))
  ;[1 1 1] Camera Movement
  ;;[1 1 1] Camera Pitching
  (if (not (`self.isDisabledCamNav`))
    (`/Engine/EditorBlueprintResources/StandardMacros.Gate` true :!label _label_3
      (:`Exit`
        (`self.K2_SetActorRotation` (`self.refCameraPawn`) (`KismetMathLibrary.MakeRotator` (.roll (`self.K2_GetActorRotation` (`self.refCameraPawn`))) (`KismetMathLibrary.FClamp` (+ (* AxisValue (`self.RotateSensitivity`)) (.pitch (`self.K2_GetActorRotation` (`self.refCameraPawn`)))) 15.0 65.0) (.yaw (`self.K2_GetActorRotation` (`self.refCameraPawn`)))) false)))))

(event `InputAction|Panning`
  (params (Key :type "Key Structure"))
  ;[1 1 1] Camera Movement
  ;;[1 1 1] Camera Pitching
  (:`Pressed`
    (goto _label_3 :!via `Open`))
  (:`Released`
    (goto _label_3 :!via `Close`)))

(fn `CalculateSensitivity`
  (returns (ReturnValue :type "Float (double-precision)"))
  (return (* (`KismetMathLibrary.FClamp` (/ (`SpringArmComponent.TargetArmLength` (`/Game/BluePrints/BP_CameraPawn.SpringArm` (`self.refCameraPawn`))) 100.0) 5.0 20.0) (`self.MoveMultiplyer`))))

(fn `GetVesselByCursor`
  (returns (Selection :type "/Game/BluePrints/Vessels/BP_BaseVessel Object Reference"))
  (bind (_worldlocation _worlddirection) (`self.DeprojectMousePositionToWorld` self))
  (bind _outhit (`KismetSystemLibrary.LineTraceSingle` _worldlocation (+ _worldlocation _worlddirection) "TraceTypeQuery4"))
  (bind _asbp_base_vessel (cast `/Game/BluePrints/Vessels/BP_BaseVessel` (`.HitActor` (`GameplayStatics.BreakHitResult` _outhit)))
    (:`then`
      (return _asbp_base_vessel))
    (:`CastFailed`
      (`KismetSystemLibrary.PrintString` "nothing under cursor"))))

(fn `SetSightDistance`
  (returns (SightDistance :type "Float (double-precision)"))
  (return (+ (`self.SightDistance`) (`SpringArmComponent.TargetArmLength` (`/Game/BluePrints/BP_CameraPawn.SpringArm` (`self.refCameraPawn`))))))

(fn `UserConstructionScript`)