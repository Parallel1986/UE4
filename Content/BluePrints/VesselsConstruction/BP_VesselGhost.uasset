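; Placement preview ghost for vessel construction, showing the selected vessel's mesh snapped to a grid at the cursor position.
; Calling a vessel briefly spawns an instance to read its display mesh and proxy, restarts the ghost with them, then destroys the instance.
; A gated Tick moves the active ghost, while spawn and kill toggle the controller's placing flag.
; It packages vessel class, proxy and transform into a struct.
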(event `OnSpawn`
  (params (DisplayMesh :type "StaticMesh Object Reference") (VesselClass :type "/Game/BluePrints/Vessels/BP_BaseVessel Class Reference") (VesselProxy :type "/Game/BluePrints/VesselsConstruction/BP_VesselProxy Class Reference"))
  ;[1 1 1] Spawn Ghost
  (if (not (`self.isActive`))
    (set `self.refDisplayMesh` DisplayMesh)
    (set `self.refBaseVessel` VesselClass)
    (set `self.refVesselProxy` VesselProxy)
    (set `self.isActive` true)
    (set `/Game/BluePrints/BP_CameraPawnController.isPlacingVessel` true (`self.refController`))
    (`StaticMeshComponent.SetStaticMesh` (`self.Vessel Ghost Mesh`) (`self.refDisplayMesh`))
    (`self.OpenTickGate`)))

(event `KillGhost`
  ;[1 1 1] Kill Ghost
  (set `self.refBaseVessel` null)
  (set `self.refVesselProxy` null)
  (set `self.refDisplayMesh` null)
  (`self.CloseTickGate`)
  (set `self.isActive` false)
  (set `/Game/BluePrints/BP_CameraPawnController.isPlacingVessel` false (`self.refController`))
  (`StaticMeshComponent.SetStaticMesh` (`self.Vessel Ghost Mesh`) (`self.refDisplayMesh`)))

(event `/Game/BluePrints/Interfaces/BP_HUD_Interface.CallVessel`
  (params (Vessel :type "/Game/BluePrints/Vessels/BP_BaseVessel Class Reference"))
  ;[1 1 1] On Vessel Call
  (bind _returnvalue (`|SpawnActorFromClass` Vessel (`KismetMathLibrary.MakeTransform` (0.0 0.0 200.0)) "Undefined" "OverrideRootScale" null (`self.refController`) null))
  (`|ExecutionSequence`
    (:`then_0`
      (bind _asbp_base_vessel (castclass `/Game/BluePrints/Vessels/BP_BaseVessel` Vessel)
        (:`then`
          (`self.KillGhost`)
          (`self.OnSpawn` (`/Game/BluePrints/Vessels/BP_BaseVessel.refDisplayMesh` _returnvalue) _asbp_base_vessel (`/Game/BluePrints/Vessels/BP_BaseVessel.refVesselProxy` _returnvalue)))
        (:`CastFailed`
          (if (!= _returnvalue null) :!label _label
            (`self.K2_DestroyActor` _returnvalue)))))
    (:`then_1`
      (goto _label))))

(event `self.ReceiveTick`
  (params (DeltaSeconds :type "Float (single-precision)"))
  ;[1 1 1] Ticking
  (`/Engine/EditorBlueprintResources/StandardMacros.Gate` true :!label _label_2
    (:`Exit`
      (`self.K2_SetActorLocation` self (`self.SetGridSnapVector`) false false))))

(event `OpenTickGate`
  ;[1 1 1] Ticking
  (goto _label_2 :!via `Open`))

(event `CloseTickGate`
  ;[1 1 1] Ticking
  (goto _label_2 :!via `Close`))

(fn `GetVesselStruct`
  (returns (VesselStructure :type "/Game/BluePrints/Structures/ST_Vessel Structure"))
  (return (make `/Game/BluePrints/Structures/ST_Vessel` (`self.refBaseVessel`) (`self.refVesselProxy`) (`KismetMathLibrary.MakeTransform` (`self.K2_GetActorLocation`) (`self.K2_GetActorRotation`)))))

(fn `Set Cursor Position`
  (params (CursorLocation :type "Vector Structure"))
  (set `self.CursorWorldPosition` CursorLocation)
  (return))

(fn `SetGridSnapVector`
  (returns (GridSnap :type "Vector Structure"))
  (bind (_cursorworldposition_x _cursorworldposition_y _cursorworldposition_z) (`KismetMathLibrary.BreakVector` (`self.CursorWorldPosition`)))
  (bind _gridsize (`self.GridSize`))
  (return (`KismetMathLibrary.MakeVector` (`/Game/BluePrints/Fuctions/Functions.Grid Snap` _cursorworldposition_x _gridsize) (`/Game/BluePrints/Fuctions/Functions.Grid Snap` _cursorworldposition_y _gridsize) (`/Game/BluePrints/Fuctions/Functions.Grid Snap` _cursorworldposition_z _gridsize))))

(fn `UserConstructionScript`)