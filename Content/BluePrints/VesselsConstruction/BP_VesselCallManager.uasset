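; BP_VesselCallManager manages calls for new vessels, spawning a placeholder proxy actor that later becomes the real vessel.
; VesselCallQueue spawns the proxy with the vessel's display mesh, binds its CallCompleted event and stores it alongside its config in parallel Proxies and Queue arrays.
; When a proxy reports completion, FinishCall looks up its config by index, removes both entries, spawns the vessel class at the stored transform and destroys the proxy.
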(event `BindCallComplete`
  (params (Proxy :type "/Game/BluePrints/VesselsConstruction/BP_VesselProxy Object Reference"))
  (add `/Game/BluePrints/VesselsConstruction/BP_VesselProxy.CallCompleted` Proxy (`|CreateDelegate` :!event `CallCompleted`)))

(event `CallCompleted`
  (params (Proxy :type "/Game/BluePrints/VesselsConstruction/BP_VesselProxy Object Reference"))
  (`self.FinishCall` Proxy))

(fn `FinishCall`
  (params (Proxy :type "/Game/BluePrints/VesselsConstruction/BP_VesselProxy Object Reference"))
  (locals (Index :type Integer :default 0) (Config :type "/Game/BluePrints/Structures/ST_Vessel Structure"))
  (bind _index (`local.Index`))
  (bind (_vesselclass _proxyclass _transform) (break `/Game/BluePrints/Structures/ST_Vessel` (`local.Config`)))
  (bind _output_get (set `local.Index` (`KismetArrayLibrary.Array_Find` (`self.Proxies`) Proxy)))
  (set `local.Config` (`|GetArrayItem` (`self.Queue`) _output_get))
  (`KismetArrayLibrary.Array_Remove` (`self.Queue`) _index)
  (`KismetArrayLibrary.Array_Remove` (`self.Proxies`) _index)
  (`|SpawnActorFromClass` _vesselclass _transform "AlwaysSpawn" "OverrideRootScale" null null null)
  (`self.K2_DestroyActor` Proxy))

(fn `UserConstructionScript`)

(fn `VesselCallQueue`
  (params (VesselStruct :type "/Game/BluePrints/Structures/ST_Vessel Structure"))
  (bind (_vesselclass _proxyclass _transform _displaymesh) (break `/Game/BluePrints/Structures/ST_Vessel` VesselStruct))
  (bind _returnvalue (`|SpawnActorFromClass` _proxyclass _transform "AlwaysSpawn" "OverrideRootScale" null _displaymesh null))
  (`self.BindCallComplete` _returnvalue)
  (`KismetArrayLibrary.Array_Add` (`self.Proxies`) _returnvalue)
  (`KismetArrayLibrary.Array_Add` (`self.Queue`) VesselStruct))