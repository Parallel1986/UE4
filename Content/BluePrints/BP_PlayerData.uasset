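; BP_PlayerData tracks which vessels the player has selected and relays target commands to them.
; A Selection array is kept in step with each object's IsSelected flag through events that clear, replace or toggle the selection.
; SetTarget passes a destination target to every selected object, and the construction script empties the array.
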(event `DeselectAll`
  ;[1 1 1] Deselect All
  (for _array_element (`self.Selection`)
    (set `/Game/BluePrints/Vessels/BP_BaseVessel.isSelected` false _array_element))
  (`KismetArrayLibrary.Array_Clear` (`self.Selection`)))

(event `SelectVessel`
  (params (SelectedObject :type "/Game/BluePrints/Vessels/BP_BaseVessel Object Reference"))
  ;[1 1 1] Add to Selection
  (`self.DeselectAll`)
  (if true
    (`KismetArrayLibrary.Array_Add` (`self.Selection`) SelectedObject)
    (set `/Game/BluePrints/Vessels/BP_BaseVessel.isSelected` true SelectedObject)))

(event `ToggleSelectionOfVessel`
  (params (SelectedObject :type "/Game/BluePrints/Vessels/BP_BaseVessel Object Reference"))
  (bind _returnvalue (`KismetArrayLibrary.Array_Find` (`self.Selection`) SelectedObject))
  ;[1 1 1] Toggle Selection
  (if (== _returnvalue -1)
    (`KismetArrayLibrary.Array_Add` (`self.Selection`) SelectedObject)
    (set `/Game/BluePrints/Vessels/BP_BaseVessel.isSelected` true SelectedObject)
    (else
      (set `/Game/BluePrints/Vessels/BP_BaseVessel.isSelected` false SelectedObject)
      (`KismetArrayLibrary.Array_Remove` (`self.Selection`) _returnvalue))))

(event `SetTarget`
  (params (DestinationTarget :type "Actor Object Reference"))
  (bind _selection (`self.Selection`))
  ;[1 1 1] Setting A Target
  (if (> (`KismetArrayLibrary.Array_Length` _selection) 0)
    (for _array_element _selection
      (`/Game/BluePrints/Vessels/BP_BaseVessel.SetTaret` _array_element DestinationTarget))))

(fn `UserConstructionScript`
  (`KismetArrayLibrary.Array_Clear` (`self.Selection`)))