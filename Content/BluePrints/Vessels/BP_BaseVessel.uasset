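; BP_BaseVessel is the base vessel actor, with a construction-set display mesh, selection feedback and a navigation target.
; On BeginPlay it spawns its own hidden BP_NavPoint, which it destroys with itself and shows or hides alongside the selection mark each Tick.
; SetTaret teleports the NavPoint to the target, keeping vessel targets and substituting the NavPoint for others.
; Steering and acceleration logic exists but is disconnected, so the vessel does not move itself.
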(event `SetTaret`
  (params (ItsTarget :type "Actor Object Reference"))
  (bind _asbp_base_vessel (cast `/Game/BluePrints/Vessels/BP_BaseVessel` ItsTarget)
    (:`then`
      (set `self.ItsTarget` _asbp_base_vessel)
      (`SceneComponent.K2_SetWorldLocation` (`/Game/BluePrints/Helpers/BP_NavPoint.Scene` (`self.NavPoint`)) (`SceneComponent.K2_GetComponentLocation` (`/Game/BluePrints/Vessels/BP_BaseVessel.Scene` _asbp_base_vessel)) false true))
    (:`CastFailed`
      (`SceneComponent.K2_SetWorldLocation` (`/Game/BluePrints/Helpers/BP_NavPoint.Scene` (`self.NavPoint`)) (`self.K2_GetActorLocation` ItsTarget) false true)
      (set `self.ItsTarget` (`self.NavPoint`)))))

(event `self.ReceiveBeginPlay`
  (bind _returnvalue (`|SpawnActorFromClass` "/Game/BluePrints/Helpers/BP_NavPoint.BP_NavPoint_C" (`KismetMathLibrary.MakeTransform` (`self.GetSelfCoordinates`)) "Undefined" "OverrideRootScale" null null null))
  (set `self.NavPoint` _returnvalue)
  (`SceneComponent.SetHiddenInGame` (`Actor.RootComponent` (`self.NavPoint`)) true false))

(event `self.ReceiveTick`
  (params (DeltaSeconds :type "Float (single-precision)"))
  (bind _navpoint (`self.NavPoint`))
  (bind _selectionmark (`self.SelectionMark`))
  (`|ExecutionSequence`
    (:`then_1`
      ;[1 1 1] Selection Checked
      (if (`self.isSelected`)
        (`SceneComponent.SetVisibility` _selectionmark true false)
        (`/Game/BluePrints/Helpers/BP_NavPoint.Show` _navpoint)
        (else
          (`SceneComponent.SetVisibility` _selectionmark false false)
          (`/Game/BluePrints/Helpers/BP_NavPoint.Hide` _navpoint))))))

(event `self.ReceiveDestroyed`
  (`self.K2_DestroyActor` (`self.NavPoint`)))

(fn `UserConstructionScript`
  (`StaticMeshComponent.SetStaticMesh` (`self.StaticMesh`) (`self.refDisplayMesh`)))